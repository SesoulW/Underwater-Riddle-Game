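; BP_Endgame is an interactable actor that plays an assigned Level Sequence, presumably the endgame sequence, when interacted with.
; Interact creates a sequence player and starts playback if the LevelSequence variable is valid.
; SetHighlight toggles the M_WaveyTexture overlay material on its static mesh, and IsInteractable returns a variable of the same name.
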(event `/Game/Blueprint/Interfaces/BPI_Puzzle.SetHighlight`
  (params (On :type Boolean))
  (`MeshComponent.SetOverlayMaterial` (`self.StaticMesh`) (select `bool` On :`true` "/Game/Materials/Overlays/M_WaveyTexture.M_WaveyTexture" :!type "MaterialInterface Object Reference")))

(event `/Game/Blueprint/Interfaces/BPI_Puzzle.Interact`
  (params (`last Possessed` :type "Pawn Object Reference"))
  (bind _level_sequence (`self.Level Sequence`))
  (`/Engine/EditorBlueprintResources/StandardMacros.IsValid` _level_sequence
    (:`Is Valid`
      (bind _outactor (`LevelSequencePlayer.CreateLevelSequencePlayer` _level_sequence))
      (`MovieSceneSequencePlayer.Play` (`LevelSequenceActor.SequencePlayer` _outactor)))))

(fn `isInteractable`
  (returns (isInteractable :type Boolean))
  (return (`self.Is Interactable`)))

(fn `UserConstructionScript`)