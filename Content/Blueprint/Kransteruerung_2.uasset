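; Interactable crane control that moves a lever and plays a Level Sequence, alternating forward and reverse on successive uses.
; It only operates when no breaches remain, fuel is present and no sequence is playing.
; A timeline animates the handle, then its finish starts the sequence and a delay tracks the playback state.
; Tick refreshes the screen text with error codes for unmet conditions, and highlighting applies an overlay material to the handle.
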(event `self.ReceiveTick`
  (params (DeltaSeconds :type "Float (single-precision)"))
  (`self.UpdateBildschirm`))

(event `self.SetHighlight`
  (params (On :type Boolean))
  (`MeshComponent.SetOverlayMaterial` (`self.Griff`) (select `bool` On :`true` "/Game/Materials/Overlays/M_WaveyTexture.M_WaveyTexture" :!type "MaterialInterface Object Reference")))

(event `self.Interact`
  (params (`last Possessed` :type "Pawn Object Reference"))
  (`|ExecutionSequence`
    (:`then_0`
      (if (== (`self.Breaches remaining`) 0)
        (set `self.A` "")
        (else
          (set `self.A` "ERROR 104")
          (`TextRenderComponent.K2_SetText` (`self.TextRender`) (`KismetTextLibrary.Conv_StringToText` (`KismetStringLibrary.Concat_StrStr` (`self.A`) " \n" (`self.B`))) :!label _label))))
    (:`then_1`
      (if (`self.is fuled`)
        (set `self.B` "")
        (else
          (set `self.B` "ERROR 404")
          (goto _label)))))
  (if (and (== (`self.Breaches remaining`) 0) (`self.is fuled`))
    (`TextRenderComponent.K2_SetText` (`self.TextRender`) (`KismetTextLibrary.Conv_StringToText` ""))
    (if (not (`self.is playing`))
      (if (not (`self.Played forward`))
        (bind (_direction _alpha) (`Timeline|Timeline` :!label _label_2)
          (:`Update`
            (`SceneComponent.K2_SetRelativeLocation` (`self.Griff`) (`KismetMathLibrary.MakeVector` 0.0 (`KismetMathLibrary.Lerp` 0.0 -14.0 _alpha) (`KismetMathLibrary.Lerp` 0.0 6.1 _alpha)) false false))
          (:`Finished`
            (bind _outactor (`LevelSequencePlayer.CreateLevelSequencePlayer` (`self.Level Sequence`)))
            (bind _sequenceplayer (`LevelSequenceActor.SequencePlayer` _outactor))
            (bind _output_get (set `self.Sequence Player` _sequenceplayer))
            (if (not (`self.Played forward`))
              (`MovieSceneSequencePlayer.Play` _output_get)
              (set `self.is playing` true)
              (bind _returnvalue (`TimeManagementBlueprintLibrary.Conv_QualifiedFrameTimeToSeconds` (`MovieSceneSequencePlayer.GetDuration` _sequenceplayer)))
              (`KismetSystemLibrary.Delay` _returnvalue)
              (set `self.is playing` false)
              (set `self.Played forward` true)
              (else
                (`MovieSceneSequencePlayer.PlayReverse` _sequenceplayer)
                (set `self.is playing` true)
                (`KismetSystemLibrary.Delay` _returnvalue)
                (set `self.is playing` false)
                (set `self.Played forward` false)))))
        (else
          (goto _label_2 :!via `Reverse`))))))

(event `UpdateBildschirm`
  (`|ExecutionSequence`
    (:`then_0`
      (if (== (`self.Breaches remaining`) 0)
        (set `self.A` "")
        (else
          (set `self.A` "ERROR 104")
          (`TextRenderComponent.K2_SetText` (`self.TextRender`) (`KismetTextLibrary.Conv_StringToText` (`KismetStringLibrary.Concat_StrStr` (`self.A`) " \n" (`self.B`))) :!label _label_3))))
    (:`then_1`
      (if (`self.is fuled`)
        (set `self.B` "")
        (else
          (set `self.B` "ERROR 404")
          (goto _label_3)))))
  (if (and (== (`self.Breaches remaining`) 0) (`self.is fuled`))
    (`TextRenderComponent.K2_SetText` (`self.TextRender`) (`KismetTextLibrary.Conv_StringToText` ""))))

(fn `isInteractable`
  (returns (isInteractable :type Boolean))
  (return (`self.Is Interactable`)))

(fn `UserConstructionScript`)