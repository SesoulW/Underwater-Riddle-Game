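; Interactable pump lever puzzle where the player pumps a barometer indicator up to a randomly placed target mark.
; Each interaction raises the indicator and swings the handle on a timeline that blocks further input until finished.
; Reaching the random pump count sets LeverIsSolved on the interacting BP_Character.
; Overshooting re-randomizes the barometer and resets BP_Button, though LeverIsSolved stays true until the next pump.
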(event `/Game/Blueprint/Interfaces/BPI_Puzzle.SetHighlight`
  (params (On :type Boolean))
  (`MeshComponent.SetOverlayMaterial` (`self.Hebelbase`) (select `bool` On :`true` "/Game/Materials/Overlays/M_WaveyTexture.M_WaveyTexture" :!type "MaterialInterface Object Reference"))
  (`MeshComponent.SetOverlayMaterial` (`self.HebelGriff`) (select `bool` On :`true` "/Game/Materials/Overlays/M_WaveyTexture.M_WaveyTexture" :!type "MaterialInterface Object Reference")))

(event `self.ReceiveBeginPlay`
  (`self.Setup_Barometer`))

(event `Setup_Barometer`
  (bind _output_get (set `self.Relative Location` (0.0 1.0 35.0)))
  (`SceneComponent.K2_SetRelativeLocation` (`self.Barometer_Duckindikator`) _output_get false false)
  (bind _output_get_2 (set `self.needed Number of pumps` (`KismetMathLibrary.RandomIntegerInRange` 3 7)))
  (`SceneComponent.K2_SetRelativeLocation` (`self.Barometer_Duckindikator_Hintergrund`) (`KismetMathLibrary.MakeVector` 0.0 0.0 (`|GetArrayItem` (`self.needed Pressure`) _output_get_2)) false false)
  (set `self.can use lever` true)
  (set `self.current Number of pumps` 0))

(event `/Game/Blueprint/Interfaces/BPI_Puzzle.Interact`
  (params (`last Possessed` :type "Pawn Object Reference"))
  (bind _needed_number_of_pumps (`self.needed Number of pumps`))
  (bind (_relative_location_x _relative_location_y _relative_location_z) (`KismetMathLibrary.BreakVector` (`self.Relative Location`)))
  (bind _bp_character (`self.BP Character`))
  (bind _asbp_character (cast `/Game/Blueprint/BP_Character` `last Possessed`))
  (set `self.BP Character` _asbp_character)
  (if (`self.can use lever`)
    (`GameplayStatics.SpawnSound2D` "/Game/Audio/Sounds/Maschinen/MS_Pump.MS_Pump" 1.0 1.0 0.0 null)
    (bind _output_get (set `self.Relative Location` (`KismetMathLibrary.MakeVector` _relative_location_x _relative_location_y (+ _relative_location_z 10.0))))
    (`SceneComponent.K2_SetRelativeLocation` (`self.Barometer_Duckindikator`) _output_get false false)
    (bind (_direction _alpha) (`Timeline|Timeline` :!via `PlayFromStart`)
      (:`Update`
        (set `self.can use lever` false)
        (`SceneComponent.K2_SetRelativeRotation` (`self.HebelGriff`) (`KismetMathLibrary.RLerp` (struct :`Pitch` 45.0) (struct :`Pitch` -45.0) _alpha) false false)
        (set `/Game/Blueprint/BP_Character.Lever is Solved` false (`self.BP Character`)))
      (:`Finished`
        (set `self.can use lever` true)
        (bind _output_get_2 (set `self.current Number of pumps` (+ (`self.current Number of pumps`) 1)))
        (if (>= _output_get_2 _needed_number_of_pumps)
          (set `/Game/Blueprint/BP_Character.Lever is Solved` true _bp_character)
          (`KismetSystemLibrary.PrintText` "Solved")
          (if (not (== _output_get_2 _needed_number_of_pumps))
            (`KismetSystemLibrary.PrintText` "to much presure")
            (`self.Setup_Barometer`)
            (bind _returnvalue (`GameplayStatics.GetActorOfClass` "/Game/Blueprint/BP_Button.BP_Button_C"))
            (`/Game/Blueprint/BP_Button.Setup Button` _returnvalue))
          (else
            (set `/Game/Blueprint/BP_Character.Lever is Solved` false _bp_character)
            (`KismetSystemLibrary.PrintText` "not Solved")))))))

(fn `isInteractable`
  (returns (isInteractable :type Boolean))
  (return (`self.Is Interactable`)))

(fn `UserConstructionScript`
  (set `self.needed Pressure` (`|MakeArray` 35.0 45.0 55.0 65.0 75.0 85.0 95.0 105.0 115.0 125.0)))