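; Possessable riddle pawn: a conductor puzzle where the player rotates cylinders into the correct sequence.
; Interact smooth-possesses it and freezes BP_Character, while possession toggles the IMC_Keypad mapping context.
; Directional input moves a highlight across the cylinder grid; interact turns the selected one 90 degrees, except both fixed end cylinders.
; Each turn compares the seven middle values, concatenated, against the solution string; a match re-possesses the player and plays a Level Sequence.
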(event `self.ReceivePossessed`
  (params (NewController :type "Controller Object Reference"))
  ;[1 0.2812 0.2812] Für alle Riddle Interactivs
  ;;[1 1 1] Toggle IMC_Keypad wenn das Keypad Posses und Unpossessed wird
  (`EnhancedInputSubsystemInterface.AddMappingContext` (pcsubsystem `EnhancedInputLocalPlayerSubsystem` (`GameplayStatics.GetPlayerController` 0)) "/Game/Inputs/Keypad/IMC_Keypad.IMC_Keypad" 0 (struct)))

(event `/Game/Blueprint/Interfaces/BPI_Puzzle.SetHighlight`
  (params (On :type Boolean))
  ;[1 0.2812 0.2812] Für alle Riddle Interactivs
  ;;[1 1 1] Toggle Highlight Material
  (`MeshComponent.SetOverlayMaterial` (`self.Board`) (select `bool` On :`true` "/Game/Materials/Overlays/M_WaveyTexture.M_WaveyTexture" :!type "MaterialInterface Object Reference")))

(event `self.ReceiveUnpossessed`
  (params (OldController :type "Controller Object Reference"))
  ;[1 0.2812 0.2812] Für alle Riddle Interactivs
  ;;[1 1 1] Toggle IMC_Keypad wenn das Keypad Posses und Unpossessed wird
  (`EnhancedInputSubsystemInterface.RemoveMappingContext` (pcsubsystem `EnhancedInputLocalPlayerSubsystem` (`GameplayStatics.GetPlayerController` 0)) "/Game/Inputs/Keypad/IMC_Keypad.IMC_Keypad" (struct)))

(event `/Game/Blueprint/Interfaces/BPI_Puzzle.Interact`
  (params (`last Possessed` :type "Pawn Object Reference"))
  ;[1 0.2812 0.2812] Für alle Riddle Interactivs
  ;;[1 1 1] Interaction mit BP_Cundoctor
  (bind _output_get (set `self.Last Possessed` `last Possessed`))
  (`|ExecutionSequence`
    (:`then_0`
      ;;;[1 1 1] Player Controller steuert/übernimmt das Keypad
      (`/Game/Blueprint/BP_MacroLibrary.MySmoothPossess` self (`self.Blend Time`))
      (bind _output_get_2 (set `self.Current Button` 0))
      (`self.SetButtonHighlight` _output_get_2))
    (:`then_1`
      ;;;[1 1 1] Ist das Object das zu letzt possed wurde der player?
      ;;; Wemm ja kann er sich der BP_Character nicht mehr bewegen
      (bind _asbp_character (cast `/Game/Blueprint/BP_Character` _output_get))
      (set `/Game/Blueprint/BP_Character.CanMove` false _asbp_character)
      (set `self.last Possessed Half Hight` (`/Game/Blueprint/BP_Character.Original Half Hight` _asbp_character)))))

(event `SetButtonHighlight`
  (params (Posiotion :type Integer) (Highlight :type Boolean))
  ;[1 1 1] Cundoctors werden highlighted
  (`/Game/Blueprint/Components/BPC_Conductor_Zylinder.SetHighlight` (`|GetArrayItem` (`self.Con_Zylinder List`) Posiotion) Highlight))

(event `AnimateButton`
  (`/Engine/EditorBlueprintResources/StandardMacros.IsValid` (`self.Last Pressed Button`)
    (:`Is Valid`
      (`SceneComponent.K2_SetRelativeRotation` :`self` (`self.Last Pressed Button`)))
    (:`Is Not Valid`
      _))
  (set `self.Last Pressed Button` null)
  ;[1 1 1] Animiert den zu letzt aktivierten Button
  (`TimelineComponent.SetPlayRate` (`self.Cundoctor Anim`) 4.0)
  (bind (_direction _alpha) (`Timeline|Cundoctor Anim` :!via `PlayFromStart`)
    (:`Update`
      (`SceneComponent.K2_SetRelativeLocation` (`self.Last Pressed Button`) (`KismetMathLibrary.MakeVector` 0.0 (`KismetMathLibrary.Lerp` 0.0 -2.0 _alpha)) false false))))

(event `EnhancedInput|/Game/Inputs/Keypad/IA_Back`
  (params (ActionValue :type Boolean) (ElapsedSeconds :type "Float (double-precision)") (TriggeredSeconds :type "Float (double-precision)") (InputAction :type "InputAction Object Reference" :default "/Game/Inputs/Keypad/IA_Back.IA_Back"))
  ;[1 1 1] Input Back
  (:`Triggered`
    (`self.Exit cundoctor`)))

(event `Exit Cundoctor`
  ;[1 1 1] Possess das letzte Object (BP_Character)
  (`self.SetButtonHighlight` (`self.Current Button`))
  (`self.DisableInput` null)
  (`/Game/Blueprint/BP_MacroLibrary.MySmoothPossess` (`self.Last Possessed`) 1.0)
  (`self.EnableInput` null))

(event `EnhancedInput|/Game/Inputs/Keypad/IA_Right`
  (params (ActionValue :type Boolean) (ElapsedSeconds :type "Float (double-precision)") (TriggeredSeconds :type "Float (double-precision)") (InputAction :type "InputAction Object Reference" :default "/Game/Inputs/Keypad/IA_Right.IA_Right"))
  ;[1 1 1] rechts
  (:`Started`
    (`self.SetButtonHighlight` (`self.Current Button`)) ; vorheriger Button wird nicht mehr highlighted
    (bind _result (`/Engine/EditorBlueprintResources/StandardMacros.IncrementInt` (`self.Current Button`)) ; Increment \nSetzt die Variable + 1\n(Aus 1 wird 2)
      (:`  `
        (if (not (< _result (`KismetArrayLibrary.Array_Length` (`self.Con_Zylinder List`))))
          (set `self.Current Button` 0) ; Button wird auf die 1. Position gesetzt
        )
        (`self.SetButtonHighlight` (`self.Current Button`) true)))))

(event `EnhancedInput|/Game/Inputs/Keypad/IA_Left`
  (params (ActionValue :type Boolean) (ElapsedSeconds :type "Float (double-precision)") (TriggeredSeconds :type "Float (double-precision)") (InputAction :type "InputAction Object Reference" :default "/Game/Inputs/Keypad/IA_Left.IA_Left"))
  ;[1 1 1] links
  (:`Started`
    (`self.SetButtonHighlight` (`self.Current Button`))
    (bind _result (`/Engine/EditorBlueprintResources/StandardMacros.DecrementInt` (`self.Current Button`)) ; Decrement\nSetzt die Variable -1\n(aus 1 wird 0)
      (:`  `
        (if (not (> _result -1))
          (bind _result_2 (`/Engine/EditorBlueprintResources/StandardMacros.DecrementInt` (`KismetArrayLibrary.Array_Length` (`self.Con_Zylinder List`)))
            (:`  `
              (set `self.Current Button` _result_2))))
        (`self.SetButtonHighlight` (`self.Current Button`) true)))))

(event `EnhancedInput|/Game/Inputs/Keypad/IA_Down`
  (params (ActionValue :type Boolean) (ElapsedSeconds :type "Float (double-precision)") (TriggeredSeconds :type "Float (double-precision)") (InputAction :type "InputAction Object Reference" :default "/Game/Inputs/Keypad/IA_Down.IA_Down"))
  (bind _returnvalue (`KismetArrayLibrary.Array_Length` (`self.Con_Zylinder List`)))
  ;[1 1 1] Down
  (:`Started`
    (`self.SetButtonHighlight` (`self.Current Button`))
    (bind _output_get (set `self.Current Button` (+ (`self.Current Button`) (`self.Cundoctors per Row`))))
    (if (not (< _output_get _returnvalue))
      (set `self.Current Button` (- (`self.Current Button`) _returnvalue)))
    (`self.SetButtonHighlight` (`self.Current Button`) true)))

(event `EnhancedInput|/Game/Inputs/Keypad/IA_Up`
  (params (ActionValue :type Boolean) (ElapsedSeconds :type "Float (double-precision)") (TriggeredSeconds :type "Float (double-precision)") (InputAction :type "InputAction Object Reference" :default "/Game/Inputs/Keypad/IA_Up.IA_Up"))
  ;[1 1 1] Up
  (:`Started`
    (`self.SetButtonHighlight` (`self.Current Button`))
    (bind _output_get (set `self.Current Button` (- (`self.Current Button`) (`self.Cundoctors per Row`))))
    (if (not (>= _output_get 0))
      (set `self.Current Button` 0))
    (`self.SetButtonHighlight` (`self.Current Button`) true)))

(event `EnhancedInput|/Game/Inputs/IA_Interact`
  (params (ActionValue :type Boolean) (ElapsedSeconds :type "Float (double-precision)") (TriggeredSeconds :type "Float (double-precision)") (InputAction :type "InputAction Object Reference" :default "/Game/Inputs/IA_Interact.IA_Interact"))
  (bind _current_button (`self.Current Button`))
  (bind _output (`|GetArrayItem` (`self.Con_Zylinder List`) (`self.Current Button`)))
  (:`Started`
    (if (== _current_button 0)
      _
      (elif (not (== _current_button 8))
        (`SceneComponent.K2_AddLocalRotation` _output (struct :`Pitch` 90.0) false false)
        (bind _output_get (set `/Game/Blueprint/Components/BPC_Conductor_Zylinder.Value` (+ (`/Game/Blueprint/Components/BPC_Conductor_Zylinder.Value` _output) 1) _output))
        (`self.Check Values`)
        (if (== _output_get 4)
          (set `/Game/Blueprint/Components/BPC_Conductor_Zylinder.Value` 0 _output))))))

(event `Check Values`
  (bind _level_sequence_to_play (`self.Level Sequence to Play`))
  (for _array_element (`self.RichtigeLösungConductors`)
    (set `self.akutelle Folge` (`KismetStringLibrary.Concat_StrStr` (`self.akutelle Folge`) (`KismetTextLibrary.Conv_TextToString` (`KismetTextLibrary.Conv_IntToText` (`/Game/Blueprint/Components/BPC_Conductor_Zylinder.Value` _array_element))))))
  (if (`KismetStringLibrary.EqualEqual_StrStr` (`self.Richtiger Folge`) (`self.akutelle Folge`))
    (`KismetSystemLibrary.PrintString` "Richtig")
    (`self.Exit Cundoctor`)
    ;[1 1 1] Play Level Sequence
    (`/Engine/EditorBlueprintResources/StandardMacros.IsValid` _level_sequence_to_play
      (:`Is Valid`
        (`MovieSceneSequencePlayer.Play` (`LevelSequenceActor.SequencePlayer` _level_sequence_to_play))))
    (else
      (`KismetSystemLibrary.PrintString` "Flasch")
      (set `self.akutelle Folge` ""))))

(fn `isInteractable`
  (returns (isInteractable :type Boolean))
  (return (`self.Is Interactable`)))

(fn `UserConstructionScript`
  (`|ExecutionSequence`
    (:`then_0`
      (set `self.RichtigeLösungConductors` (`|MakeArray` (`self.BPC_Conductor_Zylinder1`) (`self.BPC_Conductor_Zylinder2`) (`self.BPC_Conductor_Zylinder3`) (`self.BPC_Conductor_Zylinder4`) (`self.BPC_Conductor_Zylinder5`) (`self.BPC_Conductor_Zylinder6`) (`self.BPC_Conductor_Zylinder7`))))
    (:`then_1`
      (bind _output_get (set `self.Con_Zylinder List` (`|MakeArray` (`self.BPC_Conductor_Zylinder`) (`self.BPC_Conductor_Zylinder1`) (`self.BPC_Conductor_Zylinder2`) (`self.BPC_Conductor_Zylinder3`) (`self.BPC_Conductor_Zylinder4`) (`self.BPC_Conductor_Zylinder5`) (`self.BPC_Conductor_Zylinder6`) (`self.BPC_Conductor_Zylinder7`) (`self.BPC_Conductor_Zylinder8`))))
      (for _array_element _output_get
        (`PrimitiveComponent.SetMaterial` _array_element (`MeshComponent.GetMaterialIndex` _array_element "north") (`self.Material_1`))
        (`PrimitiveComponent.SetMaterial` _array_element (`MeshComponent.GetMaterialIndex` _array_element "east") (`self.Material_2`))
        (`PrimitiveComponent.SetMaterial` _array_element (`MeshComponent.GetMaterialIndex` _array_element "west") (`self.Material_3`))))))