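; Actor component that finds and highlights the puzzle interactable in front of the player's camera.
; Each Tick it sphere-traces along the camera's forward vector, accepting hits that implement BPI_Puzzle and report interactable, only while the owning Pawn is player-controlled.
; It stores the hit as CurrentInteractable, switching highlights through messages when the target changes or is lost.
; CanInteract exposes that cached actor and whether it is valid.
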(event `self.ReceiveTick`
  (params (DeltaSeconds :type "Float (single-precision)"))
  (bind _camera (`self.Camera`))
  (bind _current_interactable (`self.Current Interactable`))
  (bind _current_interactable_2 (`self.Current Interactable`))
  (bind _returnvalue (`SceneComponent.K2_GetComponentLocation` _camera))
  ;[1 1 1] Interactables werden hervorgehoben
  ;;[1 1 1] Setup Sphere Trace
  (bind _outhit (`KismetSystemLibrary.SphereTraceSingle` _returnvalue (+ _returnvalue (* (`SceneComponent.GetForwardVector` _camera) (`self.Interaction Distance`))) (`self.Interaction Radius`) "TraceTypeQuery1"))
  (bind (_bblockinghit _binitialoverlap _time _distance _location _impactpoint _normal _impactnormal _physmat _hitactor) (`GameplayStatics.BreakHitResult` _outhit))
  (bind _isinteractable (message `/Game/Blueprint/Interfaces/BPI_Puzzle.isInteractable` _hitactor))
  (if (and _isinteractable (`KismetSystemLibrary.DoesImplementInterface` _hitactor "/Game/Blueprint/Interfaces/BPI_Puzzle.BPI_Puzzle_C") (`Pawn.IsPlayerControlled` (cast `Pawn` (`self.GetOwner`) :!pure true)))
    ;;[1 1 1] ist das getroffene Object ungleich mit dem
    ;; Curent Interactable wird das alte Object nicht mehr
    ;; gehighlighted und das Neue Object wird gehighlighted wenn
    ;; die Vorraussetzungen erfüllt wurden
    (if (not (== _hitactor (`self.Current Interactable`)))
      (if (`KismetSystemLibrary.IsValid` _current_interactable_2)
        (message `/Game/Blueprint/Interfaces/BPI_Puzzle.SetHighlight` _current_interactable_2 false))
      (bind _output_get (set `self.Current Interactable` _hitactor)) ; speichhert das getroffene Object als \n"Current Interactable" Wenn es BPI_Puzzle\nbesitzt
      (message `/Game/Blueprint/Interfaces/BPI_Puzzle.SetHighlight` _output_get true))
    (else
      (`/Engine/EditorBlueprintResources/StandardMacros.IsValid` _current_interactable
        (:`Is Valid`
          (message `/Game/Blueprint/Interfaces/BPI_Puzzle.SetHighlight` _current_interactable false)
          (set `self.Current Interactable` null) ; Trifft der Trace kein Object\nOder keins mit BPI_Puzzle\nwird die Variable geleert
        )))))

(fn `Can Interact`
  (returns (`Can Interact` :type Boolean) (`Current Interactable` :type "Actor Object Reference"))
  (bind _current_interactable (`self.Current Interactable`))
  ;[1 1 1] Überprüft ob mit den gespeicherten "Current Interactable" Interagiert werden kann
  (return (`KismetSystemLibrary.IsValid` _current_interactable) _current_interactable))