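; BP_Hebel2 is an interactable, highlightable lever that acts as a step in a generator puzzle.
; When the character's button and lever checks pass, a timeline rotates the handle and toggles its on/off state.
; During animation it plays a level sequence if fuses are in place, otherwise sets the fuse box's GeneratorIsOn, with a one-time diesel pump sound.
; Failed checks reset this lever, BP_Button and BP_Hebl's barometer.
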(event `/Game/Blueprint/Interfaces/BPI_Puzzle.SetHighlight`
  (params (On :type Boolean))
  (`MeshComponent.SetOverlayMaterial` (`self.HebelBase`) (select `bool` On :`true` "/Game/Materials/Overlays/M_WaveyTexture.M_WaveyTexture" :!type "MaterialInterface Object Reference"))
  (`MeshComponent.SetOverlayMaterial` (`self.Hebelgriff`) (select `bool` On :`true` "/Game/Materials/Overlays/M_WaveyTexture.M_WaveyTexture" :!type "MaterialInterface Object Reference")))

(event `/Game/Blueprint/Interfaces/BPI_Puzzle.Interact`
  (params (`last Possessed` :type "Pawn Object Reference"))
  (bind _asbp_character (cast `/Game/Blueprint/BP_Character` `last Possessed`))
  (bind _output_get (set `self.BP Character` _asbp_character))
  (if (and (`/Game/Blueprint/BP_Character.Button is Pressed` _output_get) (`/Game/Blueprint/BP_Character.Lever is Solved` _output_get))
    (if (`self.Can use Lever`)
      (if (`self.Is ON`)
        (bind (_direction _alpha) (`Timeline|Lever_Anim` :!via `Reverse` :!label _label)
          (:`Update`
            (set `self.Can use Lever` false)
            (`SceneComponent.K2_SetRelativeRotation` (`self.Hebelgriff`) (`KismetMathLibrary.RLerp` (struct) (struct :`Pitch` -120.0) _alpha) false false)
            (if (`self.Fuses are in place`)
              (bind _outactor (`LevelSequencePlayer.CreateLevelSequencePlayer` (`self.Level Sequence`)))
              (bind _sequenceplayer (`LevelSequenceActor.SequencePlayer` _outactor))
              (`MovieSceneSequencePlayer.SetPlayRate` _sequenceplayer (`self.Play Rate`))
              (`MovieSceneSequencePlayer.Play` _sequenceplayer)
              (else
                (bind _returnvalue (`GameplayStatics.GetActorOfClass` "/Game/Blueprint/BP_Fuse_box.BP_Fuse_box_C"))
                (set `/Game/Blueprint/BP_Fuse_box.Generator is on` true _returnvalue)))
            (`/Engine/EditorBlueprintResources/StandardMacros.DoOnce` false
              (:`Completed`
                (`GameplayStatics.SpawnSoundAtLocation` "/Game/Audio/Sounds/MS_Diesel_Pump.MS_Diesel_Pump" (`SceneComponent.K2_GetComponentLocation` (`self.HebelBase`)) (struct) 1.0 1.0 0.0 null null))))
          (:`Finished`
            (set `self.Can use Lever` true)
            (if (`self.Is ON`)
              (set `self.Is ON` false)
              (else
                (set `self.Is ON` true)))))
        (else
          (goto _label))))
    (else
      (`self.Setup Lever`))))

(event `Setup Lever`
  (`SceneComponent.K2_SetRelativeRotation` :`self` (`self.Hebelgriff`))
  (set `self.Can use Lever` true)
  (set `self.Is ON` false)
  (bind _returnvalue (`GameplayStatics.GetActorOfClass` "/Game/Blueprint/BP_Button.BP_Button_C"))
  (`/Game/Blueprint/BP_Button.Setup Button` _returnvalue)
  (bind _returnvalue_2 (`GameplayStatics.GetActorOfClass` "/Game/Blueprint/BP_Hebl.BP_Hebl_C"))
  (`/Game/Blueprint/BP_Hebl.Setup_Barometer` _returnvalue_2))

(fn `isInteractable`
  (returns (isInteractable :type Boolean))
  (return true))

(fn `UserConstructionScript`)