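; BP_Schublade is an interactable drawer that slides open and closed and can carry pickups with it.
; Interact plays or reverses a timeline that moves the drawer along its relative Y axis, toggling the open state on finish.
; BP_Pickup actors overlapping the Collier component attach to the drawer on BeginPlay and begin overlap, while end overlap calls detach on the drawer component itself.
; SetHighlight toggles a wavey overlay material; a world-space slide variant remains unconnected.
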(event `/Game/Blueprint/Interfaces/BPI_Puzzle.Interact`
  (params (`last Possessed` :type "Pawn Object Reference"))
  (if (not (`self.Isopened`))
    (bind (_direction _alpha) (`Timeline|Timeline_0` :!label _label)
      (:`Update`
        (`SceneComponent.K2_SetRelativeLocation` (`self.Schublade`) (`KismetMathLibrary.MakeVector` 0.0 (+ 0.0 (`KismetMathLibrary.Lerp` 0.0 40.0 _alpha))) false false))
      (:`Finished`
        (if (`self.Isopened`)
          (set `self.Isopened` false)
          (else
            (set `self.Isopened` true)))))
    (else
      (goto _label :!via `Reverse`))))

(event `self.Collier.OnComponentEndOverlap`
  (params (OverlappedComponent :type "PrimitiveComponent Object Reference") (OtherActor :type "Actor Object Reference") (OtherComp :type "PrimitiveComponent Object Reference") (OtherBodyIndex :type Integer))
  (for _ (`self.Overlapping Actors`)
    (`SceneComponent.K2_DetachFromComponent` (`self.Schublade`) "KeepRelative" "KeepRelative" "KeepRelative" true)))

(event `self.Collier.OnComponentBeginOverlap`
  (params (OverlappedComponent :type "PrimitiveComponent Object Reference") (OtherActor :type "Actor Object Reference") (OtherComp :type "PrimitiveComponent Object Reference") (OtherBodyIndex :type Integer) (bFromSweep :type Boolean) (SweepResult :type "HitResult Structure (by ref)"))
  (bind _output_get (set `self.Overlapping Actors` (`PrimitiveComponent.GetOverlappingActors` OverlappedComponent "/Game/Blueprint/BP_Pickup.BP_Pickup_C")))
  (for _array_element _output_get
    (`self.K2_AttachToComponent` _array_element (`self.Schublade`) "None" "KeepWorld" "KeepRelative" "KeepRelative" true)))

(event `self.ReceiveBeginPlay`
  (bind _output_get (set `self.Overlapping Actors` (`PrimitiveComponent.GetOverlappingActors` (`self.Collier`) "/Game/Blueprint/BP_Pickup.BP_Pickup_C")))
  (for _array_element _output_get
    (`self.K2_AttachToComponent` _array_element (`self.Schublade`) "None" "KeepWorld" "KeepRelative" "KeepRelative" true)))

(event `/Game/Blueprint/Interfaces/BPI_Puzzle.SetHighlight`
  (params (On :type Boolean))
  (`MeshComponent.SetOverlayMaterial` (`self.Schublade`) (select `bool` On :`true` "/Game/Materials/Overlays/M_WaveyTexture.M_WaveyTexture" :!type "MaterialInterface Object Reference")))

(fn `isInteractable`
  (returns (isInteractable :type Boolean))
  (return true))

(fn `UserConstructionScript`)