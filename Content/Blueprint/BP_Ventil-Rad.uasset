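; BP_Ventil-Rad is an interactable valve wheel that plays an optional level sequence when turned.
; Interact fires once, stores the BP_Character and runs a timeline rotating the Rad mesh toward 270 degrees.
; Each timeline update also creates and plays a new sequence player if a LevelSequence is set.
; SetHighlight toggles a wavy overlay material, and IsInteractable returns a stored flag.
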(event `/Game/Blueprint/Interfaces/BPI_Puzzle.Interact`
  (params (`last Possessed` :type "Pawn Object Reference"))
  (bind _level_sequence (`self.Level Sequence`))
  (`/Engine/EditorBlueprintResources/StandardMacros.DoOnce` false
    (:`Completed`
      (bind _asbp_character (cast `/Game/Blueprint/BP_Character` `last Possessed`))
      (set `self.BP Character` _asbp_character)
      (bind (_direction _alpha) (`Timeline|Rotate Wheel`)
        (:`Update`
          (`SceneComponent.K2_SetRelativeRotation` (`self.Rad`) (`KismetMathLibrary.RLerp` (struct) (struct :`Pitch` 270.0) _alpha) false false)
          (`/Engine/EditorBlueprintResources/StandardMacros.IsValid` _level_sequence
            (:`Is Valid`
              (bind _outactor (`LevelSequencePlayer.CreateLevelSequencePlayer` _level_sequence))
              (`MovieSceneSequencePlayer.Play` (`LevelSequenceActor.SequencePlayer` _outactor)))))))))

(event `/Game/Blueprint/Interfaces/BPI_Puzzle.SetHighlight`
  (params (On :type Boolean))
  (`MeshComponent.SetOverlayMaterial` (`self.Rad`) (select `bool` On :`true` "/Game/Materials/Overlays/M_WaveyTexture.M_WaveyTexture" :!type "MaterialInterface Object Reference")))

(fn `isInteractable`
  (returns (isInteractable :type Boolean))
  (return (`self.Is Interactable`)))

(fn `UserConstructionScript`)