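; Interactable fuse box that takes held "Pickup" objects from BP_Character into three fuse slots.
; Interact, gated by a collider overlap, reveals the next fuse component and uses a Timeline lerp to move and attach the held object to that slot.
; Filling all slots plays the alarm and a second level sequence if the generator is on, otherwise flags BP_Hebel2.
; An overlay material provides highlighting, cleared on completion.
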(event `self.Collider.OnComponentBeginOverlap`
  (params (OverlappedComponent :type "PrimitiveComponent Object Reference") (OtherActor :type "Actor Object Reference") (OtherComp :type "PrimitiveComponent Object Reference") (OtherBodyIndex :type Integer) (bFromSweep :type Boolean) (SweepResult :type "HitResult Structure (by ref)"))
  (bind _asbp_character (cast `/Game/Blueprint/BP_Character` OtherActor))
  (set `self.BP Character` _asbp_character)
  (set `self.Can_Interact` true))

(event `self.Collider.OnComponentEndOverlap`
  (params (OverlappedComponent :type "PrimitiveComponent Object Reference") (OtherActor :type "Actor Object Reference") (OtherComp :type "PrimitiveComponent Object Reference") (OtherBodyIndex :type Integer))
  (cast `/Game/Blueprint/BP_Character` OtherActor)
  (set `self.Can_Interact` false))

(event `/Game/Blueprint/Interfaces/BPI_Puzzle.Interact`
  (params (`last Possessed` :type "Pawn Object Reference"))
  (bind _bp_character (`self.BP Character`))
  (bind _fuse_number (`self.Fuse_Number`))
  (bind _object_in_hand (`/Game/Blueprint/BP_Character.Object In Hand` (`self.BP Character`)))
  (bind _object_in_hand_2 (`/Game/Blueprint/BP_Character.Object In Hand` (`self.BP Character`)))
  (`/Engine/EditorBlueprintResources/StandardMacros.IsValid` (`/Game/Blueprint/BP_Character.Object In Hand` _bp_character)
    (:`Is Valid`
      (set `Widget.RenderOpacity` 0.0 (`/Game/UI/WBP_GameplayUI.Pickup_Box` (`/Game/Blueprint/Components/BPC_CheckForInteractables.WBP Gameplay UI` (`/Game/Blueprint/BP_Character.Check for Interactables` _bp_character)))))
    (:`Is Not Valid`
      _))
  (if (`self.Can_Interact`)
    (`/Engine/EditorBlueprintResources/StandardMacros.IsValid` _object_in_hand_2
      (:`Is Valid`
        (if (`self.ActorHasTag` _object_in_hand_2 "Pickup")
          (if (not (> _fuse_number 2))
            (`SceneComponent.SetHiddenInGame` (`|GetArrayItem` (`self.Fuses_Array`) _fuse_number) false false)
            (set `self.next free Pickup Loc` (`|GetArrayItem` (`self.Pickup_Los_Array`) _fuse_number))
            (set `self.Fuse_Number` (+ _fuse_number 1))
            (`/Engine/EditorBlueprintResources/StandardMacros.IsValid` _object_in_hand
              (:`Is Valid`
                (if (== (`/Game/Blueprint/BP_Pickup.Tag ` _object_in_hand) "Pickup")
                  (`self.Place Object` _object_in_hand)
                  (if (> (`self.Fuse_Number`) 2)
                    (if (`self.Generator is on`)
                      (bind (_outactor _returnvalue) (`LevelSequencePlayer.CreateLevelSequencePlayer` (`self.Level Sequence_Alarm`)))
                      (`MovieSceneSequencePlayer.Play` _returnvalue)
                      (bind _outactor_2 (`LevelSequencePlayer.CreateLevelSequencePlayer` (`self.Level Sequence to Play`)))
                      (bind _sequenceplayer (`LevelSequenceActor.SequencePlayer` _outactor_2))
                      (`MovieSceneSequencePlayer.SetPlayRate` _sequenceplayer (`self.Play Rate`))
                      (`MovieSceneSequencePlayer.Play` _sequenceplayer)
                      (else
                        (bind _returnvalue_2 (`GameplayStatics.GetActorOfClass` "/Game/Blueprint/BP_Hebel2.BP_Hebel2_C"))
                        (set `/Game/Blueprint/BP_Hebel2.Fuses are in place` true _returnvalue_2)))
                    (`MeshComponent.SetOverlayMaterial` (`self.Highlight Array`) (select `bool` false :`true` "/Game/Materials/Overlays/M_WaveyTexture.M_WaveyTexture" :!type "MaterialInterface Object Reference"))))))))))))

(event `Place Object`
  (params (`Object To Place` :type "/Game/Blueprint/BP_Pickup Object Reference"))
  (bind _bp_character (`self.BP Character`))
  ;[1 1 1] place
  (set `self.Pickup Hand Pos` (`self.K2_GetActorLocation` `Object To Place`))
  (bind (_direction _alpha) (`Timeline|Timeline` :!via `PlayFromStart`)
    (:`Update`
      (set `self.Can_Interact` false)
      (`self.K2_SetActorLocation` `Object To Place` (`KismetMathLibrary.VLerp` (`self.Pickup Hand Pos`) (`SceneComponent.K2_GetComponentLocation` (`self.next free Pickup Loc`)) _alpha) false false))
    (:`Finished`
      (bind _output_get (set `/Game/Blueprint/BP_Character.Object In Hand` `Object To Place` _bp_character))
      (`self.K2_AttachToComponent` _output_get (`self.next free Pickup Loc`) "None" "SnapToTarget" "KeepRelative" "KeepRelative" true)
      (set `/Game/Blueprint/BP_Character.Object In Hand` null _bp_character))))

(event `/Game/Blueprint/Interfaces/BPI_Puzzle.SetHighlight`
  (params (On :type Boolean))
  (`MeshComponent.SetOverlayMaterial` (`self.Highlight Array`) (select `bool` On :`true` "/Game/Materials/Overlays/M_WaveyTexture.M_WaveyTexture" :!type "MaterialInterface Object Reference")))

(fn `isInteractable`
  (returns (isInteractable :type Boolean))
  (return true))

(fn `UserConstructionScript`
  (set `self.Fuses_Array` (`|MakeArray` (`self.Fuse`) (`self.Fuse 2`) (`self.Fuse 3`)))
  (set `self.Pickup_Los_Array` (`|MakeArray` (`self.Pickup_Place`) (`self.Pickup_Place1`) (`self.Pickup_Place2`)))
  (set `self.Highlight Array` (`|MakeArray` (`self.s`) (`self.s1`) (`self.s2`) (`self.s4`) (`self.s5`) (`self.s3`))))