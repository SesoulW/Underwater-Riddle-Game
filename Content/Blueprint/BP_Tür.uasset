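; Interactable door, apparently for lockers, that swings open and closed and can show an overlay highlight material.
; Interact plays or reverses a Timeline that lerps the door mesh's yaw, and the Timeline's finish toggles IsOpened.
; The construction script applies the optional door wheel mesh and locker number and name texts, destroying those components when left unset or at "Default".
; IsInteractable exposes a flag of the same name.
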(event `/Game/Blueprint/Interfaces/BPI_Puzzle.SetHighlight`
  (params (On :type Boolean))
  (`MeshComponent.SetOverlayMaterial` (`self.Tür1`) (select `bool` On :`true` "/Game/Materials/Overlays/M_WaveyTexture.M_WaveyTexture" :!type "MaterialInterface Object Reference")))

(event `/Game/Blueprint/Interfaces/BPI_Puzzle.Interact`
  (params (`last Possessed` :type "Pawn Object Reference"))
  (if (not (`self.Is opened`))
    (bind (_direction _alpha) (`Timeline|Timeline` :!label _label)
      (:`Update`
        (`SceneComponent.K2_SetRelativeRotation` (`self.Tür1`) (`KismetMathLibrary.MakeRotator` 0.0 0.0 (`KismetMathLibrary.Lerp` 0.0 100.0 _alpha)) false false))
      (:`Finished`
        (if (`self.Is opened`)
          (set `self.Is opened` false)
          (else
            (set `self.Is opened` true)))))
    (else
      (goto _label :!via `Reverse`))))

(fn `isInteractable`
  (returns (isInteractable :type Boolean))
  (return (`self.Is Interactable`)))

(fn `UserConstructionScript`
  (bind _name (`self.Name`))
  (bind _number (`self.Number`))
  (if (not (`KismetSystemLibrary.IsValid` (`self.Türrad_Mesh`)))
    (`ActorComponent.K2_DestroyComponent` (`self.Türrad`))
    (else
      (`StaticMeshComponent.SetStaticMesh` (`self.Türrad`) (`self.Türrad_Mesh`))))
  (if (`KismetTextLibrary.EqualEqual_TextText` (`self.Locker Number`) (`KismetTextLibrary.Conv_NameToText` "Default"))
    (`ActorComponent.K2_DestroyComponent` _number)
    (else
      (`TextRenderComponent.K2_SetText` _number (`self.Locker Number`))))
  (if (`KismetTextLibrary.EqualEqual_TextText` (`self.Locker Name`) (`KismetTextLibrary.Conv_NameToText` "Default"))
    (`ActorComponent.K2_DestroyComponent` _name)
    (else
      (`TextRenderComponent.K2_SetText` _name (`self.Locker Name`)))))