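; BP_Breach is an interactable breach that the player removes with a blowtorch.
; It shows a wavy overlay material when highlighted, suppressed once in use.
; Interacting with a blowtorch-carrying BP_Character plays a slowed timeline that fades the mesh's Opacity parameter to zero.
; When finished, it decrements BreachesRemaining on the Kransteruerung_2 actor found in the level, then destroys itself after a short delay.
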(event `self.ReceiveBeginPlay`
  (`TimelineComponent.SetPlayRate` (`self.Timeline`) 0.6))

(event `/Game/Blueprint/Interfaces/BPI_Puzzle.SetHighlight`
  (params (On :type Boolean))
  (if (`self.In Useage`)
    (`MeshComponent.SetOverlayMaterial` (`self.Breach`) (select `bool` false :`true` "/Game/Materials/Overlays/M_WaveyTexture.M_WaveyTexture" :!type "MaterialInterface Object Reference"))
    (else
      (`MeshComponent.SetOverlayMaterial` (`self.Breach`) (select `bool` On :`true` "/Game/Materials/Overlays/M_WaveyTexture.M_WaveyTexture" :!type "MaterialInterface Object Reference")))))

(event `/Game/Blueprint/Interfaces/BPI_Puzzle.Interact`
  (params (`last Possessed` :type "Pawn Object Reference"))
  (bind _asbp_character (cast `/Game/Blueprint/BP_Character` `last Possessed`))
  (bind _output_get (set `self.BP Character` _asbp_character))
  (if (`/Game/Blueprint/BP_Character.Has Blowtorch` _output_get)
    (set `self.In Useage` true)
    (`MeshComponent.SetOverlayMaterial` (`self.Breach`) (select `bool` false :`true` "/Game/Materials/Overlays/M_WaveyTexture.M_WaveyTexture" :!type "MaterialInterface Object Reference"))
    (bind (_direction _alpha) (`Timeline|Timeline`)
      (:`Update`
        (`MeshComponent.SetScalarParameterValueOnMaterials` (`self.Breach`) "Opacity" (`KismetMathLibrary.Lerp` 1.0 0.0 _alpha)))
      (:`Finished`
        (bind _returnvalue (`GameplayStatics.GetActorOfClass` "/Game/Blueprint/Kransteruerung_2.Kransteruerung_2_C"))
        (set `/Game/Blueprint/Kransteruerung_2.Breaches remaining` (- (`/Game/Blueprint/Kransteruerung_2.Breaches remaining` _returnvalue) 1) _returnvalue)
        (`KismetSystemLibrary.Delay` 0.2)
        (`self.K2_DestroyActor`)))))

(fn `isInteractable`
  (returns (isInteractable :type Boolean))
  (return true))

(fn `UserConstructionScript`)