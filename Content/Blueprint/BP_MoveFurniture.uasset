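; Interactable furniture piece that rotates its cube a quarter turn once when used, then plays a level sequence.
; A highlight call toggles a wavy overlay material on the cube until the move is done.
; Interact runs through a DoOnce into a timeline that lerps the rotation.
; When the timeline finishes, it disables highlighting, clears the overlay and starts the sequence, though it still reports as interactable.
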(event `self.SetHighlight`
  (params (On :type Boolean))
  (if (not (`self.isdone`))
    (`MeshComponent.SetOverlayMaterial` (`self.Cube`) (select `bool` On :`true` "/Game/Materials/Overlays/M_WaveyTexture.M_WaveyTexture" :!type "MaterialInterface Object Reference"))))

(event `/Game/Blueprint/Interfaces/BPI_Puzzle.Interact`
  (params (`last Possessed` :type "Pawn Object Reference"))
  (`/Engine/EditorBlueprintResources/StandardMacros.DoOnce` false
    (:`Completed`
      (bind (_direction _newtrack_0) (`Timeline|Move`)
        (:`Update`
          (`SceneComponent.K2_SetRelativeRotation` (`self.Cube`) (`KismetMathLibrary.RLerp` (struct :`Roll` 90.0) (struct) _newtrack_0) false false))
        (:`Finished`
          (set `self.isdone` true)
          (`MeshComponent.SetOverlayMaterial` (`self.Cube`) (select `bool` false :`true` "/Game/Materials/Overlays/M_WaveyTexture.M_WaveyTexture" :!type "MaterialInterface Object Reference"))
          (bind _outactor (`LevelSequencePlayer.CreateLevelSequencePlayer` (`self.Level Sequence`)))
          (`MovieSceneSequencePlayer.Play` (`LevelSequenceActor.SequencePlayer` _outactor)))))))

(fn `isInteractable`
  (returns (isInteractable :type Boolean))
  (return true))

(fn `UserConstructionScript`)