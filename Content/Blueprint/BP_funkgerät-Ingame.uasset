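; Interactable handheld radio (Funkgerät) that plays random sounds in the world until the player picks it up.
; After BeginPlay it loops one of three sounds at random intervals, revealing its initially hidden screen, and highlights through an overlay material.
; Interacting with empty hands runs a sped-up timeline lerping it to the character's pickup point, then copies HasRadio to the character, plays a pickup sound and destroys the actor.
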(event `self.ReceiveBeginPlay`
  (bind _returnvalue (`self.K2_GetActorLocation`))
  (`SceneComponent.SetVisibility` (`self.Screen`) false false)
  (`TimelineComponent.SetPlayRate` (`self.Pickup Funk`) 5.0)
  (`KismetSystemLibrary.Delay` 5.0)
  (`GameplayStatics.SpawnSoundAtLocation` (`KismetArrayLibrary.Array_Random` (`self.SoundArray`)) _returnvalue (struct) 1.0 1.0 0.0 null null)
  (`KismetSystemLibrary.Delay` 5.0)
  (`KismetSystemLibrary.Delay` (`KismetMathLibrary.RandomFloatInRange` 7.0 15.0) :!label _label)
  (`GameplayStatics.SpawnSoundAtLocation` (`KismetArrayLibrary.Array_Random` (`self.SoundArray`)) _returnvalue (struct) 1.0 1.0 0.0 null null)
  (`SceneComponent.SetVisibility` (`self.Screen`) true false)
  (goto _label))

(event `self.SetHighlight`
  (params (On :type Boolean))
  (`MeshComponent.SetOverlayMaterial` (`self.Funkgerät`) (select `bool` On :`true` "/Game/Materials/Overlays/M_WaveyTexture.M_WaveyTexture" :!type "MaterialInterface Object Reference")))

(event `self.Interact`
  (params (`last Possessed` :type "Pawn Object Reference"))
  (bind _asbp_character (cast `/Game/Blueprint/BP_Character` `last Possessed`))
  (bind _output_get (set `self.Player` _asbp_character))
  (`/Engine/EditorBlueprintResources/StandardMacros.IsValid` (`/Game/Blueprint/BP_Character.Object In Hand` _output_get)
    (:`Is Not Valid`
      (if (not (`TimelineComponent.IsPlaying` (`/Game/Blueprint/BP_Character.PickupObj` _output_get)))
        (set `self.Pickup Original position` (`self.K2_GetActorLocation` self))
        (bind (_direction _alpha) (`Timeline|Pickup Funk` :!via `PlayFromStart`)
          (:`Update`
            (`self.K2_SetActorLocation` (`KismetMathLibrary.VLerp` (`self.Pickup Original position`) (`SceneComponent.K2_GetComponentLocation` (`/Game/Blueprint/BP_Character.PickupLoc` (`self.Player`))) _alpha)))
          (:`Finished`
            (`self.K2_AttachToComponent` (`/Game/Blueprint/BP_Character.PickupLoc` (`self.Player`)) "None" "SnapToTarget" "KeepRelative" "KeepRelative")
            (set `/Game/Blueprint/BP_Character.Has_Radio` (`self.Has Radio`) (`self.Player`))
            (`GameplayStatics.SpawnSound2D` "/Game/Audio/Sprecher/Pickup_funk_Sprecher.Pickup_funk_Sprecher" 1.0 1.0 0.0 null)
            (`KismetSystemLibrary.Delay` 0.2)
            (`self.K2_DestroyActor`)))))))

(fn `isInteractable`
  (returns (isInteractable :type Boolean))
  (return true))

(fn `UserConstructionScript`
  (set `self.SoundArray` (`|MakeArray` (`self.Sound`) (`self.Sound2`) (`self.Sound3`))))