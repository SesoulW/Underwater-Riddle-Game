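; BP_Keypad is a possessable, interactable riddle keypad where the player enters a code to trigger a Level Sequence.
; Interacting smooth-possesses it and freezes BP_Character, while possession toggles its input mapping context.
; Directional inputs move a wrapping highlight across the button grid, and Interact animates the button, then appends, clears or checks the code.
; A correct code exits and disables interaction, a wrong one flashes red and resets, and Back repositions and repossesses the player.
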(event `self.ReceivePossessed`
  (params (NewController :type "Controller Object Reference"))
  ;[1 0.2812 0.2812] Für alle Riddle Interactivs
  ;;[1 1 1] Toggle IMC_Keypad wenn das Keypad Posses und Unpossessed wird
  (`EnhancedInputSubsystemInterface.AddMappingContext` (pcsubsystem `EnhancedInputLocalPlayerSubsystem` (`GameplayStatics.GetPlayerController` 0)) "/Game/Inputs/Keypad/IMC_Keypad.IMC_Keypad" 0 (struct)))

(event `/Game/Blueprint/Interfaces/BPI_Puzzle.SetHighlight`
  (params (On :type Boolean))
  ;[1 0.2812 0.2812] Für alle Riddle Interactivs
  ;;[1 1 1] Toggle Highlight Material
  (`MeshComponent.SetOverlayMaterial` (`self.Keypad_Keypad-Base`) (select `bool` On :`true` "/Game/Materials/Overlays/M_WaveyTexture.M_WaveyTexture" :!type "MaterialInterface Object Reference")))

(event `self.ReceiveUnpossessed`
  (params (OldController :type "Controller Object Reference"))
  ;[1 0.2812 0.2812] Für alle Riddle Interactivs
  ;;[1 1 1] Toggle IMC_Keypad wenn das Keypad Posses und Unpossessed wird
  (`EnhancedInputSubsystemInterface.RemoveMappingContext` (pcsubsystem `EnhancedInputLocalPlayerSubsystem` (`GameplayStatics.GetPlayerController` 0)) "/Game/Inputs/Keypad/IMC_Keypad.IMC_Keypad" (struct)))

(event `/Game/Blueprint/Interfaces/BPI_Puzzle.Interact`
  (params (`last Possessed` :type "Pawn Object Reference"))
  ;[1 0.2812 0.2812] Für alle Riddle Interactivs
  ;;[1 1 1] Interaction mit BP_Keypad
  (bind _output_get (set `self.Last Possessed` `last Possessed`)) ; Übermittel das Last Possessed\nZB. den Player
  (`|ExecutionSequence`
    (:`then_0`
      ;;;[1 1 1] Player Controller steuert/übernimmt das Keypad
      (`/Game/Blueprint/BP_MacroLibrary.MySmoothPossess` self (`self.Blend Time`))
      (bind _output_get_2 (set `self.Current Button` 0))
      (`self.SetButtonHighlight` _output_get_2 true))
    (:`then_1`
      ;;;[1 1 1] Ist das Object das zu letzt possed wurde der player?
      ;;; Wemm ja kann er sich der BP_Character nicht mehr bewegen
      (bind _asbp_character (cast `/Game/Blueprint/BP_Character` _output_get))
      (set `/Game/Blueprint/BP_Character.CanMove` false _asbp_character)
      (set `self.last Possessed Capsule Half Height` (`/Game/Blueprint/BP_Character.Original Half Hight` _asbp_character)))))

(event `SetButtonHighlight`
  (params (Posiotion :type Integer) (Highlight :type Boolean))
  ;[1 1 1] Buttons werden highlighted
  (`/Game/Blueprint/Components/BPC_KeypadButton.SetHighlight` (`|GetArrayItem` (`self.ButtonList`) Posiotion) Highlight))

(event `AnimateButton`
  (`/Engine/EditorBlueprintResources/StandardMacros.IsValid` (`self.Last Pressed Button`)
    (:`Is Valid`
      (`SceneComponent.K2_SetRelativeLocation` (`self.Last Pressed Button`) (0.0 0.0 0.0) false false))
    (:`Is Not Valid`
      _))
  (set `self.Last Pressed Button` (`|GetArrayItem` (`self.ButtonList`) (`self.Current Button`)))
  ;[1 1 1] Animiert den zu letzt aktivierten Button
  (`TimelineComponent.SetPlayRate` (`self.ButtonAnim`) 4.0)
  (bind (_direction _alpha) (`Timeline|ButtonAnim` :!via `PlayFromStart`)
    (:`Update`
      (`SceneComponent.K2_SetRelativeLocation` (`self.Last Pressed Button`) (`KismetMathLibrary.MakeVector` 0.0 (`KismetMathLibrary.Lerp` 0.0 -2.0 _alpha)) false false))))

(event `EnhancedInput|/Game/Inputs/Keypad/IA_Back`
  (params (ActionValue :type Boolean) (ElapsedSeconds :type "Float (double-precision)") (TriggeredSeconds :type "Float (double-precision)") (InputAction :type "InputAction Object Reference" :default "/Game/Inputs/Keypad/IA_Back.IA_Back"))
  ;[1 1 1] Input Back
  (:`Started`
    (`self.Reposotion Player`)
    (`self.Exit Keypad`)))

(event `Exit Keypad`
  ;[1 1 1] Possess das letzte Object (BP_Character)
  (`self.SetButtonHighlight` (`self.Current Button`))
  (`self.DisableInput` null)
  (`/Game/Blueprint/BP_MacroLibrary.MySmoothPossess` (`self.Last Possessed`) 1.0)
  (`self.EnableInput` null))

(event `Reposotion Player`
  (bind _returnvalue (`SceneComponent.K2_GetComponentLocation` (`self.PlayerPos`)))
  (bind _outhit (`KismetSystemLibrary.LineTraceSingle` _returnvalue (+ _returnvalue (0.0 0.0 -250.0)) "TraceTypeQuery1"))
  (`self.K2_SetActorLocationAndRotation` (`self.Last Possessed`) (+ (`.Location` (`GameplayStatics.BreakHitResult` _outhit)) (0.0 0.0 90.0)) (`SceneComponent.K2_GetComponentRotation` (`self.PlayerPos`)) false false))

(event `EnhancedInput|/Game/Inputs/Keypad/IA_Right`
  (params (ActionValue :type Boolean) (ElapsedSeconds :type "Float (double-precision)") (TriggeredSeconds :type "Float (double-precision)") (InputAction :type "InputAction Object Reference" :default "/Game/Inputs/Keypad/IA_Right.IA_Right"))
  ;[1 1 1] rechts
  (:`Started`
    (`self.SetButtonHighlight` (`self.Current Button`)) ; vorheriger Button wird nicht mehr highlighted
    (bind _result (`/Engine/EditorBlueprintResources/StandardMacros.IncrementInt` (`self.Current Button`)) ; Increment \nSetzt die Variable + 1\n(Aus 1 wird 2)
      (:`  `
        (if (not (< _result (`KismetArrayLibrary.Array_Length` (`self.ButtonList`))))
          (set `self.Current Button` 0) ; Button wird auf die 1. Position gesetzt
        )
        (`self.SetButtonHighlight` (`self.Current Button`) true)))))

(event `EnhancedInput|/Game/Inputs/Keypad/IA_Left`
  (params (ActionValue :type Boolean) (ElapsedSeconds :type "Float (double-precision)") (TriggeredSeconds :type "Float (double-precision)") (InputAction :type "InputAction Object Reference" :default "/Game/Inputs/Keypad/IA_Left.IA_Left"))
  ;[1 1 1] links
  (:`Started`
    (`self.SetButtonHighlight` (`self.Current Button`))
    (bind _result (`/Engine/EditorBlueprintResources/StandardMacros.DecrementInt` (`self.Current Button`)) ; Decrement\nSetzt die Variable -1\n(aus 1 wird 0)
      (:`  `
        (if (not (> _result -1))
          (bind _result_2 (`/Engine/EditorBlueprintResources/StandardMacros.DecrementInt` (`KismetArrayLibrary.Array_Length` (`self.ButtonList`)))
            (:`  `
              (set `self.Current Button` _result_2))))
        (`self.SetButtonHighlight` (`self.Current Button`) true)))))

(event `EnhancedInput|/Game/Inputs/Keypad/IA_Down`
  (params (ActionValue :type Boolean) (ElapsedSeconds :type "Float (double-precision)") (TriggeredSeconds :type "Float (double-precision)") (InputAction :type "InputAction Object Reference" :default "/Game/Inputs/Keypad/IA_Down.IA_Down"))
  (bind _returnvalue (`KismetArrayLibrary.Array_Length` (`self.ButtonList`)))
  ;[1 1 1] Down
  (:`Started`
    (`self.SetButtonHighlight` (`self.Current Button`))
    (bind _output_get (set `self.Current Button` (+ (`self.Current Button`) (`self.ButtonsPerRow`))))
    (if (not (< _output_get _returnvalue))
      (set `self.Current Button` (- (`self.Current Button`) _returnvalue)))
    (`self.SetButtonHighlight` (`self.Current Button`) true)))

(event `EnhancedInput|/Game/Inputs/Keypad/IA_Up`
  (params (ActionValue :type Boolean) (ElapsedSeconds :type "Float (double-precision)") (TriggeredSeconds :type "Float (double-precision)") (InputAction :type "InputAction Object Reference" :default "/Game/Inputs/Keypad/IA_Up.IA_Up"))
  ;[1 1 1] Up
  (:`Started`
    (`self.SetButtonHighlight` (`self.Current Button`))
    (bind _output_get (set `self.Current Button` (- (`self.Current Button`) (`self.ButtonsPerRow`))))
    (if (not (>= _output_get 0))
      (set `self.Current Button` (+ (`KismetArrayLibrary.Array_Length` (`self.ButtonList`)) (`self.Current Button`))))
    (`self.SetButtonHighlight` (`self.Current Button`) true)))

(event `EnhancedInput|/Game/Inputs/IA_Interact`
  (params (ActionValue :type Boolean) (ElapsedSeconds :type "Float (double-precision)") (TriggeredSeconds :type "Float (double-precision)") (InputAction :type "InputAction Object Reference" :default "/Game/Inputs/IA_Interact.IA_Interact"))
  (bind _levelsequencetoplay (`self.LevelSequenceToPlay`))
  (bind _button (`/Game/Blueprint/Components/BPC_KeypadButton.Button` (`|GetArrayItem` (`self.ButtonList`) (`self.Current Button`))))
  ;[1 1 1] Numpad Inputs
  (:`Started`
    (`self.AnimateButton`)
    (switch `string` _button ; Überprüft welche Art Button \naktuell heighlighted ist und\n teilt den Code dementsprechend auf
      (:`Default`
        (if (< (`KismetStringLibrary.Len` (`self.CurrentCode`)) (`self.Max Code Length`))
          (bind _output_get (set `self.CurrentCode` (`KismetStringLibrary.Concat_StrStr` (`self.CurrentCode`) _button)))
          (`TextRenderComponent.K2_SetText` (`self.TXT_CurrentCode`) (`KismetTextLibrary.Conv_StringToText` _output_get))))
      (:`Confirm`
        (if (`KismetStringLibrary.EqualEqual_StrStr` (`self.CurrentCode`) (`self.Wanted`))
          ;;[1 1 1] Code ist Correct
          (`TextRenderComponent.SetTextRenderColor` (`self.TXT_CurrentCode`) (`KismetMathLibrary.LinearColor_ToRGBE` (struct :`R` 0.053049 :`G` 0.395833 :`B` 0.009807 :`A` 1.0)))
          (`self.Exit Keypad`)
          (set `self.Is Interactable` false)
          (`|ExecutionSequence`
            (:`then_0`
              ;[1 1 1] Play Level Sequence
              (`/Engine/EditorBlueprintResources/StandardMacros.IsValid` _levelsequencetoplay
                (:`Is Valid`
                  (`MovieSceneSequencePlayer.Play` (`LevelSequenceActor.SequencePlayer` _levelsequencetoplay))))))
          (else
            ;;[1 1 1] Code ist Falsch
            (`TextRenderComponent.SetTextRenderColor` (`self.TXT_CurrentCode`) (`KismetMathLibrary.LinearColor_ToRGBE` (struct :`R` 0.395833 :`B` 0.0259 :`A` 1.0)))
            (`self.DisableInput` null)
            (`KismetSystemLibrary.Delay` 1.0)
            (`self.remove Code`)
            (`self.EnableInput` null))))
      (:`Cancle`
        (`self.remove Code`)))))

(fn `isInteractable`
  (returns (isInteractable :type Boolean))
  (return (`self.Is Interactable`)))

(fn `UserConstructionScript`
  (set `self.ButtonList` (`|MakeArray` (`self.BPC_KeypadButton7`) (`self.BPC_KeypadButton8`) (`self.BPC_KeypadButton9`) (`self.BPC_KeypadButton4`) (`self.BPC_KeypadButton5`) (`self.BPC_KeypadButton6`) (`self.BPC_KeypadButton1`) (`self.BPC_KeypadButton2`) (`self.BPC_KeypadButton3`) (`self.BPC_KeypadButtonConfirm`) (`self.BPC_KeypadButton`) (`self.BPC_KeypadButtonBack`))))