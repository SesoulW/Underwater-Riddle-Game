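; Interactable double door (Tür) that swings its two leaves open or closed and shows a wavy overlay material while highlighted.
; Interact plays a random hinge sound, then runs one Timeline forward or in reverse from the end to lerp both leaves' yaw in opposite directions.
; The shared Finished handler toggles IsOpened and plays a random closing sound after closing, while IsPlaying blocks interaction mid-swing.
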(event `self.SetHighlight`
  (params (On :type Boolean))
  (`MeshComponent.SetOverlayMaterial` (`self.Tür_rechts`) (select `bool` On :`true` "/Game/Materials/Overlays/M_WaveyTexture.M_WaveyTexture" :!type "MaterialInterface Object Reference"))
  (`MeshComponent.SetOverlayMaterial` (`self.Tür_links`) (select `bool` On :`true` "/Game/Materials/Overlays/M_WaveyTexture.M_WaveyTexture" :!type "MaterialInterface Object Reference")))

(event `self.Interact`
  (params (`last Possessed` :type "Pawn Object Reference"))
  (if (not (`self.Is Playing`))
    (`GameplayStatics.PlaySoundAtLocation` (`KismetArrayLibrary.Array_Random` (`self.HingesArray`)) (`SceneComponent.K2_GetComponentLocation` (`self.DefaultSceneRoot`)) (struct) 1.0 1.0 0.0 null null null null)
    (if (not (`self.Is opened`))
      (set `self.Is Playing` true)
      (bind (_direction _alpha) (`Timeline|Timeline` :!label _label)
        (:`Update`
          (`SceneComponent.K2_SetRelativeRotation` (`self.Tür_rechts`) (`KismetMathLibrary.MakeRotator` 0.0 0.0 (`KismetMathLibrary.Lerp` 0.0 -100.0 _alpha)) false false)
          (`SceneComponent.K2_SetRelativeRotation` (`self.Tür_links`) (`KismetMathLibrary.MakeRotator` 0.0 0.0 (`KismetMathLibrary.Lerp` 0.0 90.0 _alpha)) false false))
        (:`Finished`
          (if (`self.Is opened`)
            (set `self.Is opened` false)
            (`GameplayStatics.PlaySoundAtLocation` (`KismetArrayLibrary.Array_Random` (`self.DoorClosesArray`)) (`SceneComponent.K2_GetComponentLocation` (`self.DefaultSceneRoot`)) (struct) 1.0 1.0 0.0 null null null null)
            (else
              (set `self.Is opened` true)))
          (set `self.Is Playing` false)))
      (else
        (set `self.Is Playing` true)
        (goto _label :!via `ReverseFromEnd`)))))

(fn `isInteractable`
  (returns (isInteractable :type Boolean))
  (return true))

(fn `UserConstructionScript`)