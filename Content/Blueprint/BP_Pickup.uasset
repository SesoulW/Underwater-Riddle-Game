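; BP_Pickup is an interactable actor with a fuse mesh that the player character can pick up and drop, highlighted through a wavy overlay material.
; Interact passes itself to BP_Character's PickupObject when the hand is empty and no pickup animation is playing.
; Drop detaches it and runs a sped-up timeline that lerps location to the target while applying rotation directly, then clears the character's held object.
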(event `self.ReceiveBeginPlay`
  ;[1 1 1] Timeline Speed Drop Obj
  (`TimelineComponent.SetPlayRate` (`self.DropObj`) 5.0))

(event `/Game/Blueprint/Interfaces/BPI_Puzzle.SetHighlight`
  (params (On :type Boolean))
  (`MeshComponent.SetOverlayMaterial` (`self.SM_Fuse`) (select `bool` On :`true` "/Game/Materials/Overlays/M_WaveyTexture.M_WaveyTexture" :!type "MaterialInterface Object Reference")))

(event `/Game/Blueprint/Interfaces/BPI_Puzzle.Interact`
  (params (`last Possessed` :type "Pawn Object Reference"))
  (bind _asbp_character (cast `/Game/Blueprint/BP_Character` `last Possessed`))
  (bind _output_get (set `self.Player` _asbp_character))
  (`/Engine/EditorBlueprintResources/StandardMacros.IsValid` (`/Game/Blueprint/BP_Character.Object In Hand` _output_get)
    (:`Is Not Valid`
      (if (not (`TimelineComponent.IsPlaying` (`/Game/Blueprint/BP_Character.PickupObj` _output_get)))
        (`/Game/Blueprint/BP_Character.Pickup Object` (`self.Player`) self)))))

(event `Drop`
  (params (NewLocation :type "Vector Structure") (NewRotation :type "Rotator Structure"))
  (bind (_held_location_location _held_location_rotation) (`KismetMathLibrary.BreakTransform` (`self.Held Location`)))
  (`self.K2_DetachFromActor` "KeepWorld" "KeepWorld")
  (set `self.Held Location` (`self.GetTransform`))
  (bind (_direction _alpha) (`Timeline|DropObj` :!via `PlayFromStart`)
    (:`Update`
      (`self.K2_SetActorLocationAndRotation` (`KismetMathLibrary.VLerp` _held_location_location NewLocation _alpha) NewRotation))
    (:`Finished`
      (set `/Game/Blueprint/BP_Character.Object In Hand` null (`self.Player`)))))

(fn `isInteractable`
  (returns (isInteractable :type Boolean))
  (return true))

(fn `UserConstructionScript`)