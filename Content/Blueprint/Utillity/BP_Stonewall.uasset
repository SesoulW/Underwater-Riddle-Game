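; BP_Stonewall procedurally scatters random stone meshes from the Pathstones array along an editable spline.
; The construction script steps along the spline by Gap and traces a short distance down to find the surface.
; Each hit spawns a static mesh component aligned to the surface normal, with random scale and spline-following yaw plus jitter.
; Randomness is unseeded, so the layout changes whenever construction reruns.
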(fn `UserConstructionScript`
  (bind _returnvalue (`self.GetTransform`))
  (for _index (range (+ (`KismetMathLibrary.FTrunc` (/ (`SplineComponent.GetSplineLength` (`self.Spline`)) (`self.Gap`))) 1))
    (bind _returnvalue_2 (* _index (`self.Gap`)))
    (bind _returnvalue_3 (`SplineComponent.GetLocationAtDistanceAlongSpline` (`self.Spline`) _returnvalue_2 "World"))
    (bind (_outhit _returnvalue_4) (`KismetSystemLibrary.LineTraceSingle` _returnvalue_3 (+ _returnvalue_3 (0.0 0.0 -200.0)) "TraceTypeQuery1"))
    (if _returnvalue_4
      (bind (_bblockinghit _binitialoverlap _time _distance _location _impactpoint _normal) (`GameplayStatics.BreakHitResult` _outhit))
      (bind _returnvalue_5 (`AddComponent|NODE_AddStaticMeshComponent-0` :`RelativeTransform` (`KismetMathLibrary.MakeTransform` (`KismetMathLibrary.InverseTransformLocation` _returnvalue _location) (`KismetMathLibrary.InverseTransformRotation` _returnvalue (`KismetMathLibrary.MakeRotFromZ` _normal)) (`KismetMathLibrary.VLerp` (`self.MinRandomScale`) (`self.MaxRandomScale`) (`KismetMathLibrary.RandomFloat`)))))
      (bind (_returnvalue_roll _returnvalue_pitch _returnvalue_yaw) (`KismetMathLibrary.BreakRotator` (`SplineComponent.GetRotationAtDistanceAlongSpline` (`self.Spline`) _returnvalue_2 "World")))
      (`SceneComponent.K2_AddLocalRotation` _returnvalue_5 (`KismetMathLibrary.MakeRotator` 0.0 0.0 (+ _returnvalue_yaw (`KismetMathLibrary.RandomFloatInRange` -60.0 60.0))) false false)
      ;[1 1 1] Randomisiert das gezeigt Mesh vom Array
      (`StaticMeshComponent.SetStaticMesh` _returnvalue_5 (`KismetArrayLibrary.Array_Random` (`self.Pathstones`))))))