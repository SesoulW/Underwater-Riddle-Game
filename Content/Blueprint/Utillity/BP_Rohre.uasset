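; BP_Rohre is a spline-based pipe builder ("Rohre" is German for pipes) that lays meshes along an editable path.
; The Construction Script adds one Spline Mesh Component per segment, matching its start and end positions and tangents to the neighboring spline points.
; Meshes repeat in fixed order from the first five StaticMeshes entries via index modulo.
; Each segment's up direction follows the start point's rotation to carry roll.
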(fn `UserConstructionScript`
  (bind _spline (`self.Spline`))
  (bind _spline_2 (`self.Spline`))
  (for _index (range (+ (- (`SplineComponent.GetNumberOfSplinePoints` _spline) 2) 1))
    (bind _returnvalue (`AddComponent|NODE_AddSplineMeshComponent-0`))
    (`StaticMeshComponent.SetStaticMesh` _returnvalue (`|GetArrayItem` (`self.StaticMeshes`) (mod _index 5)))
    (`SplineMeshComponent.SetSplineUpDir` _returnvalue (`KismetMathLibrary.GetUpVector` (`SplineComponent.GetRotationAtSplinePoint` (`self.Spline`) _index "Local")) true)
    (bind _returnvalue_2 (+ _index 1))
    (`SplineMeshComponent.SetStartAndEnd` _returnvalue (`SplineComponent.GetLocationAtSplinePoint` _spline _index "Local") (`SplineComponent.GetTangentAtSplinePoint` _spline _index "Local") (`SplineComponent.GetLocationAtSplinePoint` _spline_2 _returnvalue_2 "Local") (`SplineComponent.GetTangentAtSplinePoint` _spline_2 _returnvalue_2 "Local") true)))