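; Interactable crane control lever that toggles a level sequence, presumably the crane movement, forward and back.
; Interact plays or reverses the Griff timeline to shift the lever mesh, and on finish creates a new sequence player to play in the matching direction.
; IsPlaying blocks input for a fixed delay after the sequence starts, but not during lever travel.
; SetHighlight toggles an overlay material on the lever.
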(event `/Game/Blueprint/Interfaces/BPI_Puzzle.SetHighlight`
  (params (On :type Boolean))
  (`MeshComponent.SetOverlayMaterial` (`self.Hebel`) (select `bool` On :`true` "/Game/Materials/Overlays/M_WaveyTexture.M_WaveyTexture" :!type "MaterialInterface Object Reference")))

(event `/Game/Blueprint/Interfaces/BPI_Puzzle.Interact`
  (params (`last Possessed` :type "Pawn Object Reference"))
  (if (not (`self.is playing`))
    (if (not (`self.Played forward`))
      (bind (_direction _alpha) (`Timeline|Griff` :!label _label)
        (:`Update`
          (`SceneComponent.K2_SetRelativeLocation` (`self.Hebel`) (`KismetMathLibrary.MakeVector` 0.0 (`KismetMathLibrary.Lerp` 0.0 -14.0 _alpha) (`KismetMathLibrary.Lerp` 0.0 6.1 _alpha)) false false))
        (:`Finished`
          (bind _outactor (`LevelSequencePlayer.CreateLevelSequencePlayer` (`self.Level Sequence`)))
          (bind _sequenceplayer (`LevelSequenceActor.SequencePlayer` _outactor))
          (bind _output_get (set `self.Sequence Player` _sequenceplayer))
          (if (not (`self.Played forward`))
            (`MovieSceneSequencePlayer.Play` _output_get)
            (set `self.is playing` true)
            (`KismetSystemLibrary.Delay` 2.0)
            (set `self.is playing` false)
            (set `self.Played forward` true)
            (else
              (`MovieSceneSequencePlayer.PlayReverse` _sequenceplayer)
              (set `self.is playing` true)
              (`KismetSystemLibrary.Delay` 2.0)
              (set `self.is playing` false)
              (set `self.Played forward` false)))))
      (else
        (goto _label :!via `Reverse`)))))

(fn `isInteractable`
  (returns (isInteractable :type Boolean))
  (return (`self.Is Interactable`)))

(fn `UserConstructionScript`)