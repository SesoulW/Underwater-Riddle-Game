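; BP_Soundplayer is an actor that plays a configured sound, either globally in 2D or at its root component's location.
; Playback starts on BeginPlay if allowed, or when AllowPlay sets that flag and runs the same spawn logic.
; StopSound sets a stop flag, never cleared here, and re-enters the chain after the spawn to stop the stored audio component.
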(event `self.ReceiveBeginPlay`
  (bind _sound (`self.Sound`))
  (if (`self.allowed to play`) :!label _label
    (if (`self.is global`)
      (bind _returnvalue (`GameplayStatics.SpawnSound2D` _sound 1.0 1.0 0.0 null))
      (bind _output_get (set `self.sound is playing` _returnvalue :!label _label_2))
      (else
        (bind _returnvalue_2 (`GameplayStatics.SpawnSoundAtLocation` _sound (`SceneComponent.K2_GetComponentLocation` (`self.DefaultSceneRoot`)) (struct) 1.0 1.0 0.0 null null))
        (bind _output_get_2 (set `self.sound is playing` _returnvalue_2 :!label _label_3))))
    (`/Engine/EditorBlueprintResources/StandardMacros.IsValid` _output_get
      (:`Is Valid`
        (if (`self.Should stop`)
          (`AudioComponent.Stop` _output_get_2))))))

(event `AllowPlay`
  (set `self.allowed to play` true)
  (goto _label))

(event `StopSound`
  (set `self.Should stop` true)
  (if (`self.is global`)
    (goto _label_2)
    (else
      (goto _label_3))))

(fn `UserConstructionScript`)