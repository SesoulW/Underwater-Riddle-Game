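; BP_Vent is an interactable vent with a hinged door, Tür1, that opens and closes.
; Interact plays a Timeline that lerps the door's roll from 0 to 90 degrees, or reverses it when open, and toggles IsOpened on finish.
; SetHighlight applies a wavy overlay material to the door while highlighted, and IsInteractable returns a stored flag.
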(event `self.SetHighlight`
  (params (On :type Boolean))
  (`MeshComponent.SetOverlayMaterial` (`self.Tür1`) (select `bool` On :`true` "/Game/Materials/Overlays/M_WaveyTexture.M_WaveyTexture" :!type "MaterialInterface Object Reference")))

(event `self.Interact`
  (params (`last Possessed` :type "Pawn Object Reference"))
  (if (not (`self.Is opened`))
    (bind (_direction _alpha) (`Timeline|Timeline` :!label _label)
      (:`Update`
        (`SceneComponent.K2_SetRelativeRotation` (`self.Tür1`) (`KismetMathLibrary.MakeRotator` (`KismetMathLibrary.Lerp` 0.0 90.0 _alpha)) false false))
      (:`Finished`
        (if (`self.Is opened`)
          (set `self.Is opened` false)
          (else
            (set `self.Is opened` true)))))
    (else
      (goto _label :!via `Reverse`))))

(fn `isInteractable`
  (returns (isInteractable :type Boolean))
  (return (`self.Is Interactable`)))

(fn `UserConstructionScript`)