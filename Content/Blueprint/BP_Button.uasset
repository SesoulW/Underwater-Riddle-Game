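; BP_Button is an interactable puzzle button that highlights with a wavy overlay material and depends on the character's lever puzzle.
; If the lever is solved, Interact runs a timeline that lowers the cube, plays button and engine hum sounds once, then flags ButtonIsPressed on BP_Character.
; Otherwise, it calls SetupButton, which resets the cube and also sets that flag true, then runs SetupBarometer on BP_Hebl.
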(event `/Game/Blueprint/Interfaces/BPI_Puzzle.SetHighlight`
  (params (On :type Boolean))
  (`MeshComponent.SetOverlayMaterial` (`self.Cube`) (select `bool` On :`true` "/Game/Materials/Overlays/M_WaveyTexture.M_WaveyTexture" :!type "MaterialInterface Object Reference")))

(event `/Game/Blueprint/Interfaces/BPI_Puzzle.Interact`
  (params (`last Possessed` :type "Pawn Object Reference"))
  (bind _asbp_character (cast `/Game/Blueprint/BP_Character` `last Possessed`))
  (bind _output_get (set `self.BP Character` _asbp_character))
  (if (`/Game/Blueprint/BP_Character.Lever is Solved` _output_get)
    (bind (_direction _alpha) (`Timeline|Timeline`)
      (:`Update`
        (`SceneComponent.K2_SetRelativeLocation` (`self.Cube`) (`KismetMathLibrary.MakeVector` 0.0 0.0 (`KismetMathLibrary.Lerp` 0.0 -4.0 _alpha)) false false)
        (`/Engine/EditorBlueprintResources/StandardMacros.DoOnce` false
          (:`Completed`
            (`GameplayStatics.SpawnSound2D` "/Game/Audio/Sounds/Maschinen/MS_Button.MS_Button" 1.0 1.0 0.0 null)
            (`GameplayStatics.SpawnSoundAtLocation` "/Game/Audio/Sounds/Maschinen/MS_Engine_Hum.MS_Engine_Hum" (`SceneComponent.K2_GetComponentLocation` (`self.Cube`)) (struct) 1.0 1.0 0.0 null null))))
      (:`Finished`
        (set `/Game/Blueprint/BP_Character.Button is Pressed` true _output_get)))
    (else
      (`self.Setup Button`)
      (bind _returnvalue (`GameplayStatics.GetActorOfClass` "/Game/Blueprint/BP_Hebl.BP_Hebl_C"))
      (`/Game/Blueprint/BP_Hebl.Setup_Barometer` _returnvalue))))

(event `Setup Button`
  (bind _bp_character (`self.BP Character`))
  (`SceneComponent.K2_SetRelativeLocation` (`self.Cube`) (0.0 0.0 0.0) false false)
  (`/Engine/EditorBlueprintResources/StandardMacros.IsValid` _bp_character
    (:`Is Valid`
      (set `/Game/Blueprint/BP_Character.Button is Pressed` true _bp_character))))

(fn `isInteractable`
  (returns (isInteractable :type Boolean))
  (return (`self.Is Interactable`)))

(fn `UserConstructionScript`)