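; Basic game mode that sets up the game UI, music and gamma on play start, and provides player spawning and pausing.
; BeginPlay caches GI_Puzzle, builds WBP_GameUI with separate gameplay and pause stacks, and stores the PlayerStart transform.
; PlayerSpawn, not called here, possesses a new BP_Character at that transform with a camera fade.
; PauseGame toggles the pause menu, input mode and cursor, while BackoutofMessage only unpauses.
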(event `self.ReceiveBeginPlay`
  (`self.Setup Game Instance`)
  (`self.SetupUI`) ; Function (SetupUI)
  (`self.Setup Variables`)
  (`self.Play Musik`)
  (`self.Apply Gamma Value`))

(event `Setup Game Instance`
  (bind _asgi_puzzle (cast `/Game/Blueprint/GI_Puzzle` (`GameplayStatics.GetGameInstance`)))
  (set `self.Game Instance` _asgi_puzzle))

(event `Apply Gamma Value`
  (`KismetMaterialLibrary.SetScalarParameterValue` "/Game/Materials/MPC_Settings.MPC_Settings" "Gamma" (`/Game/Blueprint/GI_Puzzle.Gamma Value` (`self.Game Instance`))))

(event `Play Musik`
  (`GameplayStatics.SpawnSound2D` "/Game/Audio/Sounds/Ambients/MS_UnderwaterRoom.MS_UnderwaterRoom" 1.0 1.0 0.0 null))

(event `Player Spawn`
  (bind _spawn_transform (`self.Spawn Transform`))
  ;[1 1 1] Player Spawn
  (bind _returnvalue (`|SpawnActorFromClass` "/Game/Blueprint/BP_Character.BP_Character_C" (`KismetMathLibrary.MakeTransform` (.location _spawn_transform) (`KismetMathLibrary.MakeRotator` 0.0 0.0 (.yaw (.rotation _spawn_transform)))) "Undefined" "MultiplyWithRoot" null null))
  (`Controller.Possess` (`GameplayStatics.GetPlayerController` 0) _returnvalue)
  (`PlayerCameraManager.StartCameraFade` :`self` (`GameplayStatics.GetPlayerCameraManager` 0) :`FromAlpha` 1.0 :`Duration` 1.0 :`bHoldWhenFinished` true))

(event `Setup Variables`
  ;[1 1 1] Setup Variables
  (`|ExecutionSequence`
    (:`then_0`
      (bind _returnvalue (`GameplayStatics.GetActorOfClass` "/Script/Engine.PlayerStart"))
      (set `self.Spawn Transform` (`self.GetTransform` _returnvalue)))))

(event `PauseGame`
  (bind _returnvalue (`GameplayStatics.GetPlayerController` 0))
  (bind _pausestack (`/Game/UI/WBP_GameUI.PauseStack` (`self.GameUI`)))
  (if (not (`GameplayStatics.IsGamePaused`))
    (`CommonActivatableWidgetContainerBase.BP_AddWidget` _pausestack "/Game/UI/WBP_PauseMenuBase.WBP_PauseMenuBase_C")
    (`GameplayStatics.SetGamePaused` true)
    (`WidgetBlueprintLibrary.SetInputMode_UIOnlyEx` _returnvalue null)
    (set `PlayerController.bShowMouseCursor` true _returnvalue)
    (else
      (`CommonActivatableWidgetContainerBase.ClearWidgets` _pausestack)
      (`GameplayStatics.SetGamePaused` false)
      (`WidgetBlueprintLibrary.SetInputMode_GameOnly` _returnvalue)
      (set `PlayerController.bShowMouseCursor` false _returnvalue))))

(event `Back out of Message`
  (bind _returnvalue (`GameplayStatics.GetPlayerController` 0))
  (if (`GameplayStatics.IsGamePaused`)
    (`CommonActivatableWidgetContainerBase.ClearWidgets` (`/Game/UI/WBP_GameUI.PauseStack` (`self.GameUI`)))
    (`GameplayStatics.SetGamePaused` false)
    (`WidgetBlueprintLibrary.SetInputMode_GameOnly` _returnvalue true)
    (set `PlayerController.bShowMouseCursor` false _returnvalue)))

(fn `SetupUI`
  (bind _returnvalue (`|CreateWidget` "/Game/UI/WBP_GameUI.WBP_GameUI_C")) ; erstelle das GameUI
  (bind _output_get (set `self.GameUI` _returnvalue)) ; WBP_GameUI als Variable
  (`UserWidget.AddToViewport` _output_get 0) ; zeigt es auf den Bildschirm
  (`CommonActivatableWidgetContainerBase.BP_AddWidget` (`/Game/UI/WBP_GameUI.GameplayStack` _output_get) "/Game/UI/WBP_GameplayUI.WBP_GameplayUI_C") ; aktiviert WBP GameplayUI
)

(fn `UserConstructionScript`)