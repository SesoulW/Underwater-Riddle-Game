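; GI_Puzzle is the puzzle game's Game Instance, which applies audio volume settings at startup.
; Init calls SetupAudio, which waits one tick before overriding the SCM_Default sound mix.
; It sets the master, music, sound and dialog sound class volumes from its own volume variables, with no fade.
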(event `self.ReceiveInit`
  (`self.Setup Audio`))

(event `Setup Audio`
  (`KismetSystemLibrary.DelayUntilNextTick`)
  (`GameplayStatics.SetSoundMixClassOverride` "/Game/Audio/Settings/SCM_Default.SCM_Default" "/Game/Audio/Settings/SC_Master.SC_Master" (`self.Master Volume`) 1.0 0.0)
  (`GameplayStatics.SetSoundMixClassOverride` "/Game/Audio/Settings/SCM_Default.SCM_Default" "/Game/Audio/Settings/SC_Musik.SC_Musik" (`self.Musik Volume`) 1.0 0.0)
  (`GameplayStatics.SetSoundMixClassOverride` "/Game/Audio/Settings/SCM_Default.SCM_Default" "/Game/Audio/Settings/SC_Sound.SC_Sound" (`self.Sound Volume`) 1.0 0.0)
  (`GameplayStatics.SetSoundMixClassOverride` "/Game/Audio/Settings/SCM_Default.SCM_Default" "/Game/Audio/Settings/SC_Dialog.SC_Dialog" (`self.Dialog Volume`) 1.0 0.0))