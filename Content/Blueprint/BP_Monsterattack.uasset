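; BP_Monsterattack is a one-shot trigger that stages a monster attack scare with sound, camera shake and an optional cutscene.
; The first Collider overlap consumes a DoOnce before casting to BP_Character, then plays a located sound and shakes the camera around the character.
; A valid Sound2 adds a second located sound and gates the optional Level Sequence, which is followed three seconds later by a 2D voice line.
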(event `self.Collider.OnComponentBeginOverlap`
  (params (OverlappedComponent :type "PrimitiveComponent Object Reference") (OtherActor :type "Actor Object Reference") (OtherComp :type "PrimitiveComponent Object Reference") (OtherBodyIndex :type Integer) (bFromSweep :type Boolean) (SweepResult :type "HitResult Structure (by ref)"))
  (bind _sound_2 (`self.Sound_2`))
  (bind _level_sequence_to_play (`self.Level Sequence to Play`))
  (`/Engine/EditorBlueprintResources/StandardMacros.DoOnce` false
    (:`Completed`
      (bind _asbp_character (cast `/Game/Blueprint/BP_Character` OtherActor))
      (`GameplayStatics.SpawnSoundAtLocation` (`self.Sound`) (`SceneComponent.K2_GetComponentLocation` (`self.Soundorigine`)) (struct) 1.0 1.0 0.0 null null)
      (`GameplayStatics.PlayWorldCameraShake` "/Game/Blueprint/BP_CameraShake.BP_CameraShake_C" (`self.K2_GetActorLocation` _asbp_character) 0.0 500.0)
      (`/Engine/EditorBlueprintResources/StandardMacros.IsValid` _sound_2
        (:`Is Valid`
          (`GameplayStatics.SpawnSoundAtLocation` _sound_2 (`SceneComponent.K2_GetComponentLocation` (`self.Soundorigine2`)) (struct) 1.0 1.0 0.0 null null)
          (`/Engine/EditorBlueprintResources/StandardMacros.IsValid` _level_sequence_to_play
            (:`Is Valid`
              (bind _outactor (`LevelSequencePlayer.CreateLevelSequencePlayer` _level_sequence_to_play))
              (`MovieSceneSequencePlayer.Play` (`LevelSequenceActor.SequencePlayer` _outactor))
              (`KismetSystemLibrary.Delay` 3.0)
              (`GameplayStatics.SpawnSound2D` (`self.Sound-Voicactor`) 1.0 1.0 0.0 null))))))))

(fn `UserConstructionScript`)